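; Player hero character with Sekiro-style grappling hook, target lock-on and finishing moves on a posture-broken boss.
; Tick sphere-traces for grapple points, rejecting blocked ones; on input, a second trace validates footing, then timelines move the cable, with separate events flying the player.
; Holding left mouse triggers executions through montages and player-bound Level Sequences, varying by boss life points.
; Tick also raises hazard warnings and eases the delayed health bar.
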(event Custom|StartGrapplingEvent
  (Pawn|Components|CharacterMovement|SetMovementMode (Variables|Character|GetCharacterMovement) "MOVE_Flying" 0)
  (Components|Movement|StopMovementImmediately (Variables|Character|GetCharacterMovement))
  (Variables|Default|SetActorCurrentLocation (Transformation|GetActorLocation))
  (CallFunction|GrappleCalculatePlayerGrappleTargetLocation)
  (bind _1 (Timeline|GrappleMoveActorTimeline PlayFromStart)
    (:Update
      (CallFunction|GrappleSetActorLocationFunc _1)
      (Variables|Default|SetIsGrappling false))
    (:Finished
      (CallFunction|EndGrappleSwitchStates))))

(event Custom|EndGrappleSwitchStates
  (Pawn|Components|CharacterMovement|SetMovementMode (Variables|Character|GetCharacterMovement) "MOVE_Falling" 0)
  (Variables|Default|SetIsGrappling false)
  (Variables|/Script/Engine.CharacterMovementComponent|SetGravityScale (Variables|Character|GetCharacterMovement) 1.75))

(event Custom|EndGrapplingEvent
  (Variables|/Script/CableComponent.CableComponent|SetbAttachStart (Variables|/Game/REF/BluePrintsPlayer/BP_Cable.BP_Cable_C|GetCable (Variables|Default|GetBPCable)) false)
  (Variables|Default|SetIsGrappling false))

(event Custom|ActivateCineCamera
  (Game|Player|SetViewTargetwithBlend (Game|GetPlayerController 0) 0 1.0 "VTBlend_Linear" 0.0 false))

(event Custom|MoveCameraToOriginalLocation
  (params (Montage :type Anim%20Montage%20Object%20Reference) (bInterrupted :type Boolean))
  (bind _springarm (Variables|Default|GetSpringArm))
  ;[1 1 1] 원래 카메라로 복귀
  (if (== Montage "/Game/Blueprints/Animation/Player/ReAM_LastKill.ReAM_LastKill")
    (bind _newtrack_0 (Timeline|Timeline_1 PlayFromStart)
      (:Update
        (bind _returnvalue (CallFunction|EaseOutQuint _newtrack_0))
        (Transformation|SetRelativeTransform (Variables|Default|GetCamera) (Math|Transform|Lerp(Transform) (Transformation|GetRelativeTransform (Variables|Default|GetCamera)) (Variables|Default|GetOriginaltransfrom) _returnvalue) false false))
      (:Finished
        (Transformation|DetachFromComponent _springarm "KeepWorld" "KeepWorld" "KeepWorld" true)
        (Transformation|AttachComponentToComponent _springarm (Variables|Default|GetArrow4) "None" "SnapToTarget" "SnapToTarget" "SnapToTarget" true)))))

(event Custom|LastKillSequence
  (bind (_outactor _returnvalue) (Sequencer|Player|CreateLevelSequencePlayer "/Game/REF/BluePrintsPlayer/LevelSeqeunce/LSQ_AttackAnim.LSQ_AttackAnim"))
  (Variables|/Script/LevelSequence.LevelSequenceActor|SetbOverrideInstanceData _outactor true)
  (bind _asdefault_level_sequence_instance_data (Utilities|Casting|CastToDefaultLevelSequenceInstanceData (Variables|/Script/LevelSequence.LevelSequenceActor|GetDefaultInstanceData _outactor)))
  (Variables|/Script/LevelSequence.DefaultLevelSequenceInstanceData|SetTransformOrigin _asdefault_level_sequence_instance_data (Transformation|GetActorTransform))
  (Class|LevelSequenceActor|SetBindingbyTag _outactor "Player" (Utilities|Array|MakeArray self) false)
  (Sequencer|Player|Play _returnvalue :!class /Script/MovieScene.MovieSceneSequencePlayer))

(event Custom|FirstKillSequence
  (bind (_outactor _returnvalue) (Sequencer|Player|CreateLevelSequencePlayer "/Game/REF/BluePrintsPlayer/LevelSeqeunce/Attack_Sequence.Attack_Sequence"))
  (Variables|/Script/LevelSequence.LevelSequenceActor|SetbOverrideInstanceData _outactor true)
  (bind _asdefault_level_sequence_instance_data (Utilities|Casting|CastToDefaultLevelSequenceInstanceData (Variables|/Script/LevelSequence.LevelSequenceActor|GetDefaultInstanceData _outactor)))
  (Variables|/Script/LevelSequence.DefaultLevelSequenceInstanceData|SetTransformOrigin _asdefault_level_sequence_instance_data (Transformation|GetActorTransform))
  (Class|LevelSequenceActor|SetBindingbyTag _outactor "Player" (Utilities|Array|MakeArray self) false)
  (Sequencer|Player|Play _returnvalue :!class /Script/MovieScene.MovieSceneSequencePlayer))

(event Input|EnhancedActionEvents|EnhancedInputAction
  (params (ActionValue :type Boolean) (ElapsedSeconds :type Float%20%28double-precision%29) (TriggeredSeconds :type Float%20%28double-precision%29) (InputAction :type Input%20Action%20Object%20Reference :default "IA_Hook"))
  (bind _returnvalue (Transformation|GetActorRotation))
  (if (not (Variables|Default|GetIsGrappling))
    (if (Variables|Default|GetDidHit)
      ;[1 1 1] 걸을 수 잇는 표면이 있는지 확인
      (if (CallFunction|GrappleTargetInfo)
        ;[1 1 1] 너무 가까우면 안돼용
        (if (<= (Variables|Default|GetDistance) 2e+02)
          (Development|PrintString "Target Too Close")
          (else
            (Rendering|SetActorHiddenInGame (Variables|Default|GetBPCable) false)
            (Variables|/Script/CableComponent.CableComponent|SetbAttachStart (Variables|/Game/REF/BluePrintsPlayer/BP_Cable.BP_Cable_C|GetCable (Variables|Default|GetBPCable)) true)
            (Variables|Default|SetIsGrappling true)
            ;[1 1 1] 그랩위치의 z축 쳐다보기
            (Transformation|SetActorRotation (Math|Rotator|MakeRotator (.roll _returnvalue) (.pitch _returnvalue) (.yaw (Variables|Default|GetGrappleTargetRotation))))
            ;[1 1 1] 케이블을 이동
            (Variables|Default|SetCurrentActorLocation (Transformation|GetActorLocation))
            (Variables|/Script/Engine.CharacterMovementComponent|SetGravityScale (Variables|Character|GetCharacterMovement) 0.5)
            (bind _0_50 (Timeline|GrappleMoveCableTimeLine PlayFromStart)
              (:Update
                (CallFunction|GrappleSetCableLocation _0_50))
              (:Finished
                (Rendering|SetActorHiddenInGame (Variables|Default|GetBPCable) true)
                (Development|PrintString "Hello")))))
        (else
          (Development|PrintString "notarget")))
      (else
        (Development|PrintString "NoTarget")))))

(event Input|EnhancedActionEvents|EnhancedInputAction
  (params (ActionValue :type Boolean) (ElapsedSeconds :type Float%20%28double-precision%29) (TriggeredSeconds :type Float%20%28double-precision%29) (InputAction :type Input%20Action%20Object%20Reference :default "IA_TargetLock"))
  (bind _targetlockon (Variables|Default|GetTargetLockOn))
  (if (Variables|/Game/REF/BluePrintsPlayer/TargetLockOn.TargetLockOn_C|GetLockon (Variables|Default|GetTargetLockOn))
    (Default|StopTargetLockon _targetlockon)
    (else
      (Default|TriggerTargetLockon _targetlockon))))

(event EventBeginPlay
  ;[1 1 1] 시작할때 cable 붙이기
  (bind _returnvalue (Game|SpawnActorfromClass "/Game/REF/BluePrintsPlayer/BP_Cable.BP_Cable_C" (Transformation|GetActorTransform) "Undefined" "MultiplyWithRoot" 0 0))
  (bind _output_get (Variables|Default|SetBPCable _returnvalue))
  (Rendering|SetActorHiddenInGame _output_get true)
  (bind _asbp_isekiro_game_mode_base (Utilities|Casting|CastTo (Game|GetGameMode)))
  (bind _returnvalue_2 (CallFunction|GetMainUI _asbp_isekiro_game_mode_base))
  (bind _output_get_2 (Variables|Default|SetCharacterWidget _returnvalue_2))
  (bind _aswbp_character_widget (Utilities|Casting|CastTo _output_get_2))
  (Variables|Default|SetWBPChracterWidget _aswbp_character_widget)
  (bind _returnvalue_3 (CallFunction|GetRealHpBar (Variables|Default|GetCharacterWidget)))
  (bind _output_get_3 (Variables|Default|SetRealHpBar _returnvalue_3))
  (bind _aswbp_health_bar (Utilities|Casting|CastTo _output_get_3))
  (bind _output_get_4 (Variables|Default|SetAs%20WBP%20Health%20Bar _aswbp_health_bar))
  (Variables|Default|SetCUrrentFGHealth (Variables|Default|GetFGValueEnd _output_get_4)))

(event EventTick
  (params (DeltaSeconds :type Float%20%28single-precision%29))
  (bind (_start _end) (|CollapseGraph_2_2))
  (bind _as_wbp_health_bar (Variables|Default|GetAs%20WBP%20Health%20Bar))
  (bind _mesh (Variables|Character|GetMesh))
  (bind _returnvalue (Components|SkeletalMesh|GetAnimInstance _mesh))
  (bind _fgvalueend (Variables|Default|GetFGValueEnd _as_wbp_health_bar))
  ;[1 1 1] Tick
  (Utilities|FlowControl|Sequence
    (:then_0
      ;[1 1 1] 매 틱마다 와이어액션할 곳 트레이싱 & 너무 가까우면 표시되지 않음
      (if (not (Variables|Default|GetIsGrappling))
        (bind (_outhit _returnvalue_2) (Collision|SphereTraceByChannel _start _end 8e+02 "TraceTypeQuery3" false 0 "None" true "(R=0.903094,G=1.000000,B=0.006859,A=1.000000)" "(R=0.787162,G=0.634080,B=1.000000,A=1.000000)"))
        (if _returnvalue_2
          (bind (_outhit_2 _returnvalue_3) (Collision|LineTraceByChannel (.ImpactPoint (Collision|BreakHitResult _outhit)) (Transformation|GetActorLocation) "TraceTypeQuery1" false 0 "None"))
          (if _returnvalue_3
            (Variables|Default|SetDidHit false)
            (Utilities|ResetWire)
            (else
              (Variables|Default|SetDidHit true)
              (if (== (.HitActor (Collision|BreakHitResult _outhit)) (.hitactor (Variables|Default|GetFirstTrace)))
                (bind _output_get (Variables|Default|SetFirstTrace _outhit))
                (bind _asbp_actor (Utilities|Casting|CastToBP_Actor (.hitactor _output_get)))
                (Variables|/Game/REF/BluePrintsPlayer/BP_Actor.BP_Actor_C|SetbIsFocused _asbp_actor true)
                (else
                  (bind _asbp_actor_2 (Utilities|Casting|CastToBP_Actor (.hitactor (Variables|Default|GetFirstTrace)))
                    (:then
                      (Variables|/Game/REF/BluePrintsPlayer/BP_Actor.BP_Actor_C|SetbIsFocused _asbp_actor_2 false))
                    (:CastFailed
                      _))
                  (bind _output_get_2 (Variables|Default|SetFirstTrace _outhit))
                  (if (>= (Math|Vector|Distance(Vector) (.ImpactPoint (Collision|BreakHitResult _output_get_2)) (Transformation|GetActorLocation)) 6e+02)
                    (bind _asbp_actor_3 (Utilities|Casting|CastToBP_Actor (.HitActor (Collision|BreakHitResult _output_get_2))))
                    (Variables|/Game/REF/BluePrintsPlayer/BP_Actor.BP_Actor_C|SetbIsFocused _asbp_actor_3 true))))))
          (else
            (Utilities|ResetWire)))))
    (:then_1
      (if (and (not (Variables|Default|GetbHasDisplayedHazardUI)) (Utilities|Enum|Equal(Enum) (Variables|Default|GetHazardState) 0))
        (Variables|Default|SetbHasDisplayedHazardUI true)
        (bind _returnvalue_4 (UserInterface|CreateWidget "/Game/REF/BluePrintsPlayer/WBP_HazardState.WBP_HazardState_C" 0 self 2.8e+02))
        ;[1 1 1] 인살 준비 카메라무브
        (UserInterface|Viewport|AddtoViewport _returnvalue_4 0)
        (Audio|PlaySound2D "/Game/Assets/Sound/Combat/Sekiro_-_Perilous_Attack_Sound_Effect.Sekiro_-_Perilous_Attack_Sound_Effect" 1.0 1.0 0.0 0 0)
        (elif (and (Variables|Default|GetbHasDisplayedHazardUI) (Utilities|Enum|Equal(Enum) (Variables|Default|GetHazardState) 0))
          (Variables|Default|SetbHasDisplayedHazardUI false))))
    (:then_2
      (bind _returnvalue_5 (Actor|GetActorOfClass 0))
      (if (CallFunction|IsPostureBroken (Actor|GetComponentbyClass _returnvalue_5 0))
        (if (== (CallFunction|GetLifePoints (Actor|GetComponentbyClass _returnvalue_5 0)) 1)
          (CallFunction|SetBlur (Variables|Default|GetWBPChracterWidget))
          (if (Variables|Default|GetToExecute?)
            (Utilities|FlowControl|Sequence
              (:then_0
                (Animation|Montage|MontagePlay _returnvalue "/Game/Blueprints/Animation/Player/AM_IfBossHas1HPPoint.AM_IfBossHas1HPPoint" 1.0 "MontageLength" 0.0 true)
                (bind _returnvalue_6 (Actor|GetActorOfClass 0))
                (bind _output_get_3 (Variables|Default|SetAs%20BP%20Boss%20Test%203 _returnvalue_6))
                (CallFunction|SetLockonTarget _output_get_3 false)
                (bind _newtrack_0 (Timeline|Timeline_3 PlayFromStart)
                  (:Update
                    (Transformation|SetActorLocation (Math|Vector|Lerp(Vector) (Transformation|GetActorLocation) (+ (Transformation|GetActorLocation _output_get_3) (* (Transformation|GetActorRightVector _output_get_3) 75.0)) _newtrack_0) false false))
                  (:Finished
                    (bind _newtrack_0_2 (Timeline|Timeline_4 PlayFromStart)
                      (:Update
                        (Transformation|SetActorLocation (Math|Vector|Lerp(Vector) (Transformation|GetActorLocation) (+ (* (Transformation|GetActorForwardVector _output_get_3) -75.0) (Transformation|GetActorLocation _output_get_3)) _newtrack_0_2) false false))))))
              (:then_1
                (CallFunction|LastKillSequence))
              (:then_2
                (CallFunction|SetBlurBack (Variables|Default|GetWBPChracterWidget)))))
          (elif (Variables|Default|GetToExecute?)
            (Variables|Default|SetOriginaltransfrom (Transformation|GetRelativeTransform (Variables|Default|GetCamera)))
            (Animation|Montage|MontagePlay _returnvalue "/Game/Blueprints/Animation/Player/ReAM_LastKill.ReAM_LastKill" 1.0 "MontageLength" 0.0 true)
            (CallFunction|FirstKillSequence)))))
    (:then_3
      (if (and (!= _fgvalueend (Variables|Default|GetCUrrentFGHealth)) (not (Variables|Default|GetbIsDirty)))
        (Variables|Default|SetbIsDirty true)
        (bind _newtrack_0_3 (Timeline|BGHealthTimeLine PlayFromStart)
          (:Update
            (Variables|Default|SetBGEnd _as_wbp_health_bar (Math|Float|Lerp (Variables|Default|GetCUrrentFGHealth) _fgvalueend _newtrack_0_3)))
          (:Finished
            (Variables|Default|SetCUrrentFGHealth (Variables|Default|GetFGValueEnd _as_wbp_health_bar))
            (Variables|Default|SetbIsDirty false)))))))

(event Input|KeyboardEvents|0
  (params (Key :type Key%20Structure))
  (:Pressed
    (Animation|Montage|PlayMontage (Variables|Character|GetMesh) 0
      (:then
        (bind _returnvalue (Game|SpawnActorfromClass "/Game/REF/BluePrintsPlayer/BP_CameraAnimation.BP_CameraAnimation_C" (Math|Transform|MakeTransform "0, 0, 0") "Undefined" "MultiplyWithRoot" 0 0))
        (Default|PlayCameraAnim _returnvalue)
        (Default|EndCameraAnimation _returnvalue)))))

(event Input|MouseEvents|MouseWheelDown
  (params (Key :type Key%20Structure))
  (:Pressed
    (Default|SwitchTargetonRight (Variables|Default|GetTargetLockOn))))

(event Input|KeyboardEvents|2
  (params (Key :type Key%20Structure))
  (:Pressed
    (Transformation|SetActorLocation (Variables|Default|GetBPCable) (Transformation|GetActorLocation) false false)))

(event Input|MouseEvents|LeftMouseButton
  (params (Key :type Key%20Structure))
  ;[1 1 1] 인살 준비 카메라무브
  (:Pressed
    (Variables|Default|SetToExecute? true))
  (:Released
    (Variables|Default|SetToExecute? false)))

(event Input|KeyboardEvents|8
  (params (Key :type Key%20Structure))
  (:Pressed
    (CallFunction|ActivateCineCamera)))

(event Input|MouseEvents|MouseWheelUp
  (params (Key :type Key%20Structure))
  (:Pressed
    (Default|SwitchTargetonLeft (Variables|Default|GetTargetLockOn))))

(event Input|KeyboardEvents|5
  (params (Key :type Key%20Structure))
  (:Pressed
    (Animation|Montage|MontagePlay (Components|SkeletalMesh|GetAnimInstance (Variables|Character|GetMesh)) "/Game/Blueprints/Animation/Player/AM_IfBossHas1HPPoint.AM_IfBossHas1HPPoint" 1.0 "MontageLength" 0.0 true)))

(fn ConstructionScript)

(fn GrappleTargetInfo
  (bind _firsttrace (Variables|Default|GetFirstTrace))
  (bind _impactpoint (Collision|BreakHitResult _firsttrace))
  ;[1 1 1] 딛고 설 표면이 있는지 확인
  (bind (_outhit _returnvalue) (Collision|SphereTraceForObjects (+ _impactpoint "0.000000,0.000000,33.000000") (+ _impactpoint "0.000000,0.000000,-30.000000") 33.0 (Utilities|Array|MakeArray "ObjectTypeQuery1") false 0 "None" true "(R=0.000000,G=1.000000,B=0.519073,A=1.000000)" "(R=0.000000,G=1.000000,B=0.405393,A=1.000000)"))
  (if _returnvalue
    (bind _output_get (Variables|Default|SetSecondTrace _outhit))
    (CallFunction|GrappleGetTargetTransform _output_get)
    (return _returnvalue)))

(fn GrappleGetTargetTransform
  (params (SecondTraceRes :type Hit%20Result%20Structure))
  (Variables|Default|SetGrappleTargetLocation (.ImpactPoint (Collision|BreakHitResult SecondTraceRes)))
  (Variables|Default|SetGrappleTargetRotation (Math|Rotator|FindLookatRotation (Transformation|GetActorLocation) (Variables|Default|GetGrappleTargetLocation)))
  (Variables|Default|SetDistance (Math|Vector|Distance(Vector) (Variables|Default|GetGrappleTargetLocation) (Transformation|GetActorLocation)))
  (return))

(fn GrappleSetCableLocation
  (params (Alpha :type Float%20%28double-precision%29))
  (Transformation|SetActorLocation (Variables|Default|GetBPCable) (Math|Vector|Lerp(Vector) (Transformation|GetActorLocation) (+ (Variables|Default|GetGrappleTargetLocation) (Math|Vector|MakeVector 0.0 0.0 -5.0)) Alpha) false false))

(fn GrappleCalculatePlayerGrappleTargetLocation
  (bind _returnvalue (Transformation|GetActorForwardVector))
  (bind _secondtrace (Variables|Default|GetSecondTrace))
  (bind _impactpoint (Collision|BreakHitResult _secondtrace))
  (bind _returnvalue_2 (* _returnvalue -111.0))
  (bind _returnvalue_3 (+ _returnvalue_2 _impactpoint))
  (Variables|Default|SetTargetLocation (Math|Vector|MakeVector (.x _returnvalue_3) (.y _returnvalue_3) (+ (.z _returnvalue_3) 1e+02)))
  (return))

(fn GrappleSetActorLocationFunc
  (params (Alpha :type Float%20%28double-precision%29))
  (bind _returnvalue (Transformation|GetActorLocation))
  (bind _targetlocation (Variables|Default|GetTargetLocation))
  (bind _returnvalue_2 (+ _targetlocation (Math|Vector|MakeVector 0.0 0.0 -5.0)))
  (bind _returnvalue_3 (Math|Vector|Lerp(Vector) _returnvalue _returnvalue_2 Alpha))
  (Transformation|SetActorLocation (Math|Vector|MakeVector (.x _returnvalue_3) (.y _returnvalue_3) (.z _returnvalue_3)) false false))

(fn StartHitStop
  (params (Duration :type Float%20%28double-precision%29))
  (Variables|Default|SetCustomTimeDilation 0.0)
  (Utilities|Time|SetTimerbyFunctionName 0 "EndHitStop" Duration))

(fn EndHitStop
  (Variables|Default|SetCustomTimeDilation 1.0))

(fn UpdateHealthValue
  (params (NewFGHealth :type Float%20%28double-precision%29)))

(fn SetHealth)