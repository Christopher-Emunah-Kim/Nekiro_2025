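; BP_Actor is a grapple point that shows a WBP_GrappleUI widget while it is focused.
; It creates the widget on BeginPlay with itself as target, and Tick adds or removes it as IsFocused changes until IsGrappled is set.
; StartGrapple notifies the widget and sets that flag.
; EnableWireSpot switches the lock-on collision between Block and Overlap on a custom trace channel.
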(event EventBeginPlay
  (bind _returnvalue (UserInterface|CreateWidget "/Game/REF/BluePrintsPlayer/WBP_GrappleUI.WBP_GrappleUI_C" 0 self 5e+01))
  (Variables|Default|SetGrappleWidget _returnvalue))

(event EventTick
  (params (DeltaSeconds :type Float%20%28single-precision%29))
  (if (not (Variables|Default|GetbIsGrappled))
    (if (and (Variables|Default|GetbIsFocused) (not (UserInterface|Viewport|IsinViewport (Variables|Default|GetGrappleWidget))))
      (UserInterface|Viewport|AddtoViewport (Variables|Default|GetGrappleWidget) 0)
      (elif (and (not (Variables|Default|GetbIsFocused)) (UserInterface|Viewport|IsinViewport (Variables|Default|GetGrappleWidget)))
        (Widget|RemovefromParent (Variables|Default|GetGrappleWidget))))))

(fn ConstructionScript)

(fn EnableWireSpot
  (params (bEnable :type Boolean))
  (if bEnable
    (Collision|SetCollisionResponsetoChannel (Variables|Default|Getlockoncollision) "ECC_GameTraceChannel2" "ECR_Block")
    (else
      (Collision|SetCollisionResponsetoChannel (Variables|Default|Getlockoncollision) "ECC_GameTraceChannel2" "ECR_Overlap"))))

(fn StartGrapple
  (Default|StartGrapple (Variables|Default|GetGrappleWidget))
  (Variables|Default|SetbIsGrappled true))